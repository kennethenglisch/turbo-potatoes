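; PickUpKey is a key pickup Blueprint that flags when the player is close enough to interact and shows a prompt widget.
; BoxCollision overlaps with the cached FirstPersonCharacter toggle CanInteract and the widget's visibility.
; A looping timer, rather than Tick, turns the widget toward the player on yaw only.
; The pickup action itself is not handled in these graphs.
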(event `self.ReceiveBeginPlay`
  (`|ExecutionSequence`
    (:`then_0`
      (bind _asfirst_person_character (cast `/Game/FirstPersonBP/Blueprints/FirstPersonCharacter` (`GameplayStatics.GetPlayerCharacter` 0)))
      (set `self.Player Character` _asfirst_person_character)
      (`SceneComponent.SetVisibility` (`self.Widget`) false false))
    (:`then_1`
      ;[1 1 1] Widget always faces to the player
      (`KismetSystemLibrary.K2_SetTimerDelegate` (delegate `Spin`) 0.1 true))))

(event `Spin`
  (bind _widget (`self.Widget`))
  (bind (_returnvalue_roll _returnvalue_pitch _returnvalue_yaw) (`KismetMathLibrary.BreakRotator` (`KismetMathLibrary.FindLookAtRotation` (`SceneComponent.K2_GetComponentLocation` _widget) (`SceneComponent.K2_GetComponentLocation` (`Character.CapsuleComponent` (`self.Player Character`))))))
  ;[1 1 1] Widget always faces to the player
  (`SceneComponent.K2_SetWorldRotation` _widget (`KismetMathLibrary.MakeRotator` 0.0 0.0 _returnvalue_yaw) false false))

(event `self.Box Collision.OnComponentBeginOverlap`
  (params (OverlappedComponent :type "PrimitiveComponent Object Reference") (OtherActor :type "Actor Object Reference") (OtherComp :type "PrimitiveComponent Object Reference") (OtherBodyIndex :type Integer) (bFromSweep :type Boolean) (SweepResult :type "HitResult Structure (by ref)"))
  ;[1 1 1] Check if can interact / player in range of object
  (if (== OtherActor (`self.Player Character`))
    (set `self.canInteract` true)
    (`SceneComponent.SetVisibility` (`self.Widget`) true false)))

(event `self.Box Collision.OnComponentEndOverlap`
  (params (OverlappedComponent :type "PrimitiveComponent Object Reference") (OtherActor :type "Actor Object Reference") (OtherComp :type "PrimitiveComponent Object Reference") (OtherBodyIndex :type Integer))
  ;[1 1 1] Check if can interact / player in range of object
  (if (== (`self.Player Character`) OtherActor)
    (set `self.canInteract` false)
    (`SceneComponent.SetVisibility` (`self.Widget`) false false)))

(fn `UserConstructionScript`)