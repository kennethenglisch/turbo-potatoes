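; Locked door actor that swings open once unlocked, with key-dependent prompts for the player.
; Box overlap checks the first-person character's key count, sets CanBeOpened and shows an open or key-needed widget, removed on exit.
; Tick polls IsUnlocked, which is not set here, then stops player tracing, clears the mesh's tags and calls OpenDoor.
; A timeline drives door yaw up to MaxDoorAngle; CloseDoor reverses it.
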(event `self.ReceiveBeginPlay`
  (`|ExecutionSequence`
    (:`then_0`
      (bind _asfirst_person_character (cast `/Game/FirstPersonBP/Blueprints/FirstPersonCharacter` (`GameplayStatics.GetPlayerCharacter` 0)))
      (set `self.Player Character` _asfirst_person_character))))

(event `self.ReceiveTick`
  (params (DeltaSeconds :type "Float (single-precision)"))
  (if (`self.isUnlocked`)
    (`/Game/FirstPersonBP/Blueprints/FirstPersonCharacter.StopTracing` (`self.Player Character`))
    (`KismetArrayLibrary.Array_Clear` (`ActorComponent.ComponentTags` (`self.SM_Door`)))
    (`self.OpenDoor`)))

(event `self.Box Collision.OnComponentBeginOverlap`
  (params (OverlappedComponent :type "PrimitiveComponent Object Reference") (OtherActor :type "Actor Object Reference") (OtherComp :type "PrimitiveComponent Object Reference") (OtherBodyIndex :type Integer) (bFromSweep :type Boolean) (SweepResult :type "HitResult Structure (by ref)"))
  (bind _player_character (`self.Player Character`))
  (if (== OtherActor _player_character)
    (if (`self.isUnlocked`)
      _
      (elif (>= (`/Game/FirstPersonBP/Blueprints/FirstPersonCharacter.NumberOfKeys` _player_character) 1)
        (`KismetSystemLibrary.PrintString` "Door can open")
        (set `self.canBeOpened` true)
        (bind _returnvalue (`|CreateWidget` "/Game/Blueprints/OpenDoorWidget.OpenDoorWidget_C"))
        (`UserWidget.AddToViewport` _returnvalue 0)
        (else
          (`KismetSystemLibrary.PrintString` "You need keys")
          (set `self.canBeOpened` false)
          (bind _returnvalue_2 (`|CreateWidget` "/Game/Blueprints/KeyNeededWidget.KeyNeededWidget_C" (`GameplayStatics.GetPlayerController` 0)))
          (`UserWidget.AddToViewport` _returnvalue_2 0))))))

(event `self.Box Collision.OnComponentEndOverlap`
  (params (OverlappedComponent :type "PrimitiveComponent Object Reference") (OtherActor :type "Actor Object Reference") (OtherComp :type "PrimitiveComponent Object Reference") (OtherBodyIndex :type Integer))
  (if (== OtherActor (`self.Player Character`))
    (set `self.canBeOpened` false)
    (bind _foundwidgets (`WidgetBlueprintLibrary.GetAllWidgetsOfClass` "/Game/Blueprints/KeyNeededWidget.KeyNeededWidget_C"))
    (bind _output (`|GetArrayItem` _foundwidgets))
    (if (`KismetSystemLibrary.IsValid` _output)
      (`Widget.RemoveFromParent` _output))
    (bind _foundwidgets_2 (`WidgetBlueprintLibrary.GetAllWidgetsOfClass` "/Game/Blueprints/OpenDoorWidget.OpenDoorWidget_C"))
    (bind _output_2 (`|GetArrayItem` _foundwidgets_2))
    (if (`KismetSystemLibrary.IsValid` _output_2)
      (`Widget.RemoveFromParent` _output_2))))

(event `OpenDoor`
  (bind (_direction _newtrack_0) (`Timeline|Timeline_0` :!label _label)
    (:`Update`
      (`SceneComponent.K2_SetRelativeRotation` (`self.SM_Door`) (`KismetMathLibrary.MakeRotator` 0.0 0.0 (* _newtrack_0 (`self.maxDoorAngle`))) false false))))

(event `CloseDoor`
  (goto _label :!via `Reverse`))

(fn `UserConstructionScript`)