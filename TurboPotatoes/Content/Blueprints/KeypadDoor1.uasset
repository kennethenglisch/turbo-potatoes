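; Keypad-locked door that generates a random four-digit code at BeginPlay and scatters its digits, with positions, across four shuffled KeypadCodeBook actors.
; It binds to the KeypadUI code-entered event, and CheckCode compares entries to the code, unlocking and swinging the door open via a timeline with sound on a match.
; A box collider toggles the player's keypad section and shows or removes the enter-code prompt widget.
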(event `self.ReceiveBeginPlay`
  (`self.CreateCorrectCode`)
  (bind _asfirst_person_character (cast `/Game/FirstPersonBP/Blueprints/FirstPersonCharacter` (`GameplayStatics.GetPlayerCharacter` 0)))
  (set `self.PlayerCharacter` _asfirst_person_character)
  (bind _askeypad_ui (cast `/Game/Blueprints/KeypadUI` (`WidgetComponent.GetUserWidgetObject` (`self.KeypadWidget`))))
  (bind _output_get (set `self.KeyPadUI` _askeypad_ui))
  (add `/Game/Blueprints/KeypadUI.CodeEntered` _output_get (`|CreateDelegate` :!event `CheckCode`)))

(event `self.BoxCollider.OnComponentBeginOverlap`
  (params (OverlappedComponent :type "PrimitiveComponent Object Reference") (OtherActor :type "Actor Object Reference") (OtherComp :type "PrimitiveComponent Object Reference") (OtherBodyIndex :type Integer) (bFromSweep :type Boolean) (SweepResult :type "HitResult Structure (by ref)"))
  (if (== OtherActor (`self.PlayerCharacter`))
    (`/Game/FirstPersonBP/Blueprints/FirstPersonCharacter.ActivateKeypadCodeSection` (`self.PlayerCharacter`))
    (if (`self.isUnlocked`)
      (`KismetSystemLibrary.PrintString` "Door can open")
      (set `self.canBeOpened` true)
      (else
        (`KismetSystemLibrary.PrintString` "need to enter code")
        (set `self.canBeOpened` false)
        (bind _returnvalue (`|CreateWidget` "/Game/Blueprints/EnterCodeWidget.EnterCodeWidget_C" (`GameplayStatics.GetPlayerController` 0)))
        (`UserWidget.AddToViewport` _returnvalue 0)))
    (else
      (`KismetSystemLibrary.PrintString` "wrong player1"))))

(event `self.BoxCollider.OnComponentEndOverlap`
  (params (OverlappedComponent :type "PrimitiveComponent Object Reference") (OtherActor :type "Actor Object Reference") (OtherComp :type "PrimitiveComponent Object Reference") (OtherBodyIndex :type Integer))
  (if (== OtherActor (`self.PlayerCharacter`))
    (`/Game/FirstPersonBP/Blueprints/FirstPersonCharacter.DeactivateKeypadCodeSection` (`self.PlayerCharacter`))
    (set `self.canBeOpened` false)
    (bind _foundwidgets (`WidgetBlueprintLibrary.GetAllWidgetsOfClass` "/Game/Blueprints/EnterCodeWidget.EnterCodeWidget_C"))
    (bind _output (`|GetArrayItem` _foundwidgets))
    (if (`KismetSystemLibrary.IsValid` _output)
      (`Widget.RemoveFromParent` _output))
    (else
      (`KismetSystemLibrary.PrintString` "wrong player"))))

(event `OpenDoor`
  (`GameplayStatics.PlaySoundAtLocation` "/Game/Sounds/open_door_squeak.open_door_squeak" (`self.K2_GetActorLocation`) (struct) 0.75 1.0 0.0 null null null)
  (bind (_direction _newtrack_0) (`Timeline|door movement` :!label _label)
    (:`Update`
      (`SceneComponent.K2_SetRelativeRotation` (`self.Door`) (`KismetMathLibrary.MakeRotator` 0.0 0.0 (* _newtrack_0 (`self.maxDoorAngle`))) false false))))

(event `CloseDoor`
  (goto _label :!via `Reverse`))

(fn `CheckCode`
  (params (CodeEntered :type String) (KeypadUI :type "/Game/Blueprints/KeypadUI Object Reference"))
  (if (`KismetStringLibrary.EqualEqual_StrStr` CodeEntered (`self.CorrectCode`))
    (set `self.isUnlocked` true)
    (`self.OpenDoor`)
    (set `/Game/Blueprints/KeypadUI.CurrentCode` "" (`self.KeyPadUI`))
    (else
      (set `self.isUnlocked` false)
      (set `/Game/Blueprints/KeypadUI.CurrentCode` "" (`self.KeyPadUI`))
      (`KismetSystemLibrary.PrintString` "wrong code"))))

(fn `CreateCorrectCode`
  (locals (firstDigit :type Integer) (secondDigit :type Integer) (thirdDigit :type Integer) (fourthDigit :type Integer) (CreatedCode :type String) (KeypadBooks :type "Array of /Game/Blueprints/KeypadCodeBook Object Reference") (codeKeyDigits :type "Array of Integer"))
  (bind _returnvalue (`KismetMathLibrary.RandomIntegerInRange` 0 9))
  (bind _keypadbooks (`local.KeypadBooks`))
  (bind _output_get (set `local.firstDigit` _returnvalue))
  (bind _output_get_2 (set `local.secondDigit` _returnvalue))
  (bind _output_get_3 (set `local.thirdDigit` _returnvalue))
  (bind _output_get_4 (set `local.fourthDigit` _returnvalue))
  (bind _output_get_5 (set `local.CreatedCode` (`KismetStringLibrary.Concat_StrStr` (`KismetStringLibrary.Conv_IntToString` _output_get) (`KismetStringLibrary.Conv_IntToString` _output_get_2) (`KismetStringLibrary.Conv_IntToString` _output_get_3) (`KismetStringLibrary.Conv_IntToString` _output_get_4))))
  (`KismetSystemLibrary.PrintString` (`KismetStringLibrary.Concat_StrStr` "CREATED CODE: " _output_get_5) true true (struct :`G` 0.66 :`B` 1.0 :`A` 1.0) 10.0)
  (set `self.CorrectCode` _output_get_5)
  (bind _outactors (`GameplayStatics.GetAllActorsOfClass` "/Game/Blueprints/KeypadCodeBook.KeypadCodeBook_C"))
  (bind _output_get_6 (set `local.KeypadBooks` _outactors))
  (bind _returnvalue_2 (`KismetArrayLibrary.Array_Length` _output_get_6))
  (if (== _returnvalue_2 4)
    (set `local.codeKeyDigits` (`|MakeArray` (`local.firstDigit`) (`local.secondDigit`) (`local.thirdDigit`) (`local.fourthDigit`)))
    (`KismetArrayLibrary.Array_Shuffle` _keypadbooks)
    (for (_array_element _array_index) _keypadbooks
      ;[1 1 1] For Each Book assign randomly code parts
      (set `/Game/Blueprints/KeypadCodeBook.codePart` (`KismetStringLibrary.Conv_IntToString` (`|GetArrayItem` (`local.codeKeyDigits`) _array_index)) _array_element)
      (set `/Game/Blueprints/KeypadCodeBook.codePartIndex` _array_index _array_element))
    (else
      (`KismetSystemLibrary.PrintString` (`KismetStringLibrary.Concat_StrStr` "ERROR: FOUND " (`KismetStringLibrary.Conv_IntToString` _returnvalue_2) " BOOKS FOR THE CODE INSTEAD OF 4")))))

(fn `UserConstructionScript`)