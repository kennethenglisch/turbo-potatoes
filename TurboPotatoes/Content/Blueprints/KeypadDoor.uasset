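; Keypad-locked door that swings open when the correct code is entered on its widget-component keypad UI.
; BeginPlay caches the first-person character and binds to the keypad's code-entered event.
; CheckCode compares the entry, clears it, and on a match unlocks and plays a timeline scaling door yaw to a maximum angle.
; A box overlap sets a can-open flag for the player when unlocked, but nothing here reads it or calls CloseDoor.
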(event `self.ReceiveBeginPlay`
  (bind _asfirst_person_character (cast `/Game/FirstPersonBP/Blueprints/FirstPersonCharacter` (`GameplayStatics.GetPlayerCharacter` 0)))
  (set `self.PlayerCharacter` _asfirst_person_character)
  (bind _askeypad_ui (cast `/Game/Blueprints/KeypadUI` (`WidgetComponent.GetUserWidgetObject` (`self.KeypadWidget`))))
  (bind _output_get (set `self.KeyPadUI` _askeypad_ui))
  (add `/Game/Blueprints/KeypadUI.CodeEntered` _output_get (`|CreateDelegate` :!event `CheckCode`)))

(event `self.BoxCollider.OnComponentBeginOverlap`
  (params (OverlappedComponent :type "PrimitiveComponent Object Reference") (OtherActor :type "Actor Object Reference") (OtherComp :type "PrimitiveComponent Object Reference") (OtherBodyIndex :type Integer) (bFromSweep :type Boolean) (SweepResult :type "HitResult Structure (by ref)"))
  (if (== OtherActor (`self.PlayerCharacter`))
    (if (`self.isUnlocked`)
      (`KismetSystemLibrary.PrintString` "Door can open")
      (set `self.canBeOpened` true)
      (else
        (`KismetSystemLibrary.PrintString` "need to enter code")
        (set `self.canBeOpened` false)))
    (else
      (`KismetSystemLibrary.PrintString` "wrong player1"))))

(event `self.BoxCollider.OnComponentEndOverlap`
  (params (OverlappedComponent :type "PrimitiveComponent Object Reference") (OtherActor :type "Actor Object Reference") (OtherComp :type "PrimitiveComponent Object Reference") (OtherBodyIndex :type Integer))
  (if (== OtherActor (`self.PlayerCharacter`))
    (set `self.canBeOpened` false)
    (else
      (`KismetSystemLibrary.PrintString` "wrong player"))))

(event `OpenDoor`
  (bind (_direction _newtrack_0) (`Timeline|door movement` :!label _label)
    (:`Update`
      (`SceneComponent.K2_SetRelativeRotation` (`self.Door`) (`KismetMathLibrary.MakeRotator` 0.0 0.0 (* _newtrack_0 (`self.maxDoorAngle`))) false false))))

(event `CloseDoor`
  (goto _label :!via `Reverse`))

(fn `CheckCode`
  (params (CodeEntered :type String) (KeypadUI :type "/Game/Blueprints/KeypadUI Object Reference"))
  (if (`KismetStringLibrary.EqualEqual_StrStr` CodeEntered (`self.CorrectCode`))
    (set `self.isUnlocked` true)
    (`self.OpenDoor`)
    (set `/Game/Blueprints/KeypadUI.CurrentCode` "" (`self.KeyPadUI`))
    (else
      (set `self.isUnlocked` false)
      (set `/Game/Blueprints/KeypadUI.CurrentCode` "" (`self.KeyPadUI`))
      (`KismetSystemLibrary.PrintString` "wrong code"))))

(fn `UserConstructionScript`)