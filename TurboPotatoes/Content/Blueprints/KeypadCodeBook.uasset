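; Keypad code book actor that holds one code part and its index, and shows an interact prompt when the player is near.
; BeginPlay caches the first-person character and prints the code part and index for debugging.
; Box overlap with the player toggles CanInteract, creating the interact widget on entry and removing the first one found by class on exit.
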(event `self.ReceiveBeginPlay`
  ;[1 1 1] Setting Player Character
  (bind _asfirst_person_character (cast `/Game/FirstPersonBP/Blueprints/FirstPersonCharacter` (`GameplayStatics.GetPlayerCharacter` 0)))
  (set `self.Player Character` _asfirst_person_character)
  (`KismetSystemLibrary.PrintString` (`KismetStringLibrary.Concat_StrStr` "Code part: " (`self.codePart`) ", codePartIndex: " (`KismetStringLibrary.Conv_IntToString` (`self.codePartIndex`))) true true (struct :`G` 0.66 :`B` 1.0 :`A` 1.0) 10.0))

(event `self.Box Collision.OnComponentBeginOverlap`
  (params (OverlappedComponent :type "PrimitiveComponent Object Reference") (OtherActor :type "Actor Object Reference") (OtherComp :type "PrimitiveComponent Object Reference") (OtherBodyIndex :type Integer) (bFromSweep :type Boolean) (SweepResult :type "HitResult Structure (by ref)"))
  ;[1 1 1] Handling Widget Activation and Deactivation
  (if (== OtherActor (`self.Player Character`))
    (set `self.canInteract` true)
    (bind _returnvalue (`|CreateWidget` "/Game/Blueprints/InteractWidget.InteractWidget_C" (`GameplayStatics.GetPlayerController` 0)))
    (`UserWidget.AddToViewport` _returnvalue 0)))

(event `self.Box Collision.OnComponentEndOverlap`
  (params (OverlappedComponent :type "PrimitiveComponent Object Reference") (OtherActor :type "Actor Object Reference") (OtherComp :type "PrimitiveComponent Object Reference") (OtherBodyIndex :type Integer))
  ;[1 1 1] Handling Widget Activation and Deactivation
  (if (== (`self.Player Character`) OtherActor)
    (set `self.canInteract` false)
    (bind _foundwidgets (`WidgetBlueprintLibrary.GetAllWidgetsOfClass` "/Game/Blueprints/InteractWidget.InteractWidget_C"))
    (`Widget.RemoveFromParent` (`|GetArrayItem` _foundwidgets))))

(fn `UserConstructionScript`)